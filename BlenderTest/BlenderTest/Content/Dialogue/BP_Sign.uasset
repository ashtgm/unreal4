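; BP_Sign is an interactable sign that shows a "Press E to Interact" prompt near the player and starts dialogue when used.
; On BeginPlay it creates an Interact_UI widget and adds it to the viewport.
; Its Box trigger sets or clears the prompt text as BP_ThirdPersonCharacter enters or leaves.
; The Interact event calls Speak on its BPCDialogue component to run the dialogue.
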(event `/Game/Assets/Models/Lever/BPI_Interact.Interact`
  ; Make the Speak work
  (`/Game/Dialogue/BPC_Dialogue.Speak` (`self.BPC_Dialogue`)))

(event `self.Box.OnComponentBeginOverlap`
  (params (OverlappedComponent :type "PrimitiveComponent Object Reference") (OtherActor :type "Actor Object Reference") (OtherComp :type "PrimitiveComponent Object Reference") (OtherBodyIndex :type Integer) (bFromSweep :type Boolean) (SweepResult :type "HitResult Structure (by ref)"))
  (cast `/Game/ThirdPerson/Blueprints/BP_ThirdPersonCharacter` OtherActor)
  (`TextBlock.SetText` (`/Game/Blueprints/UI/Interact_UI.TextBlock_0` (`self.TextBox`)) "Press \"E\" to Interact"))

(event `self.Box.OnComponentEndOverlap`
  (params (OverlappedComponent :type "PrimitiveComponent Object Reference") (OtherActor :type "Actor Object Reference") (OtherComp :type "PrimitiveComponent Object Reference") (OtherBodyIndex :type Integer))
  (cast `/Game/ThirdPerson/Blueprints/BP_ThirdPersonCharacter` OtherActor)
  (`TextBlock.SetText` (`/Game/Blueprints/UI/Interact_UI.TextBlock_0` (`self.TextBox`)) ""))

(event `self.ReceiveBeginPlay`
  (bind _returnvalue (`|CreateWidget` "/Game/Blueprints/UI/Interact_UI.Interact_UI_C" (`GameplayStatics.GetPlayerController` 0)))
  (bind _output_get (set `self.TextBox` _returnvalue))
  (`UserWidget.AddToViewport` _output_get 0))

(fn `UserConstructionScript`)