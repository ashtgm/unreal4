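; Skybox actor that displays a configurable sky texture on a static mesh, set up entirely in the construction script.
; It creates a dynamic instance of M_skybox, passes in SkyTexture and converts the FollowsCamera flag into the material's "Follows Camera" scalar.
; The texture parameter and material slot names are both None.
; IsRound selects the mesh, though both options are named Skybox; the event graph is inactive.
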(fn `UserConstructionScript`
  (`|ExecutionSequence`
    (:`then_0`
      (bind _returnvalue (`PrimitiveComponent.CreateDynamicMaterialInstance` (`self.StaticMesh`) 0 "/Game/Assets/Models/Skybox/M_skybox.M_skybox" "None"))
      (`MaterialInstanceDynamic.SetTextureParameterValue` _returnvalue "None" (`self.Sky Texture`))
      (`MaterialInstanceDynamic.SetScalarParameterValue` _returnvalue "Follows Camera" (`KismetMathLibrary.SelectFloat` 1.0 0.0 (`self.Follows Camera`)))
      (`PrimitiveComponent.SetMaterialByName` (`self.StaticMesh`) "None" _returnvalue))
    (:`then_1`
      (`StaticMeshComponent.SetStaticMesh` (`self.StaticMesh`) (select `bool` (`self.Is Round`) :`false` "/Game/Assets/Models/Skybox/skybox.skybox" :`true` "/Game/Assets/Models/Skybox/skybox.skybox" :!type "StaticMesh Object Reference")))))